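; Zombie enemy that wanders, moves toward the player on sight and loses health to projectiles.
; Projectile overlaps reduce health, destroying it at zero or spawning an impact effect and issuing a move with no target set.
; PawnSensing starts the chase, while Tick issues delayed random roaming moves whenever CanSeePlayer is false.
; CanSeePlayer is only ever set false here, so sighting never suspends roaming through that flag.
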(event `self.ReceiveActorBeginOverlap`
  (params (OtherActor :type "Actor Object Reference"))
  ;[1 1 1] Taking damage from bullet
  (bind _asprojectile_base (cast `/Game/Blueprints/Projectile_Base` OtherActor))
  (set `self.Zombie1 Health` (- (`self.Zombie1 Health`) 0.2))
  (if (<= (`self.Zombie1 Health`) 0.0)
    (`self.K2_DestroyActor`)
    (else
      (`GameplayStatics.SpawnEmitterAtLocation` "/Game/InfinityBladeEffects/Effects/FX_Mobile/Impacts/P_Impact_Shield_Fire.P_Impact_Shield_Fire" (`self.K2_GetActorLocation` _asprojectile_base))
      (cast `/Game/ThirdPersonBP/Blueprints/PlayerCharacter` (`GameplayStatics.GetPlayerCharacter` 0))
      (`|AIMoveTo` self (0.0 0.0 0.0) null))))

(event `self.ReceiveTick`
  (params (DeltaSeconds :type "Float (single-precision)"))
  ;[1 1 1] Chase player
  (if (not (`self.CanSeePlayer`))
    (`KismetSystemLibrary.Delay` 3.0)
    (`|AIMoveTo` self (`NavigationSystemV1.K2_GetRandomReachablePointInRadius` (`self.K2_GetActorLocation`) 5000.0 null null) null)))

(event `self.PawnSensing.OnSeePawn`
  (params (Pawn :type "Pawn Object Reference"))
  ;[1 1 1] Chase player
  (bind _asplayer_character (cast `/Game/ThirdPersonBP/Blueprints/PlayerCharacter` Pawn))
  (set `self.CanSeePlayer` false)
  (`|AIMoveTo` self (0.0 0.0 0.0) _asplayer_character
    (:`OnSuccess`
      _)
    (:`OnFail`
      _))
  (set `self.CanSeePlayer` false))

(fn `UserConstructionScript`)